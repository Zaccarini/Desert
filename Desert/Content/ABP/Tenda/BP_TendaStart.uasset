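; VR start trigger, likely a curtain, that moves the player from the starting room into the landscape through a warp transition.
; A motion controller overlapping its Box hides the actor and, after a short delay, fires a DoOnce-guarded teleport that also turns off overlap events.
; The timed sequence shows two warp actors, lifts the pawn high up, swaps room for landscape, then lowers the pawn, respawns BpDrappo and hides the warps.
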(event `self.Box.OnComponentBeginOverlap`
  (params (OverlappedComponent :type "PrimitiveComponent Object Reference") (OtherActor :type "Actor Object Reference") (OtherComp :type "PrimitiveComponent Object Reference") (OtherBodyIndex :type Integer) (bFromSweep :type Boolean) (SweepResult :type "HitResult Structure (by ref)"))
  (cast `/Game/VirtualRealityBP/Blueprints/BP_MotionController` OtherActor)
  (cast `/Game/VirtualRealityBP/Blueprints/MotionControllerPawn` (`GameplayStatics.GetPlayerPawn` 0))
  (`self.SetActorHiddenInGame` true)
  (`KismetSystemLibrary.Delay` 0.2)
  (`/Engine/EditorBlueprintResources/StandardMacros.DoOnce` false :!label _label
    (:`Completed`
      (`self.TeleportFromStart`)
      (`KismetSystemLibrary.Delay` 5.0)
      (goto _label :!via `Reset`))))

(event `TeleportFromStart`
  (set `PrimitiveComponent.bGenerateOverlapEvents` false (`self.Box`))
  (`self.SetActorHiddenInGame` (`self.Warp1`) false)
  (`self.SetActorHiddenInGame` (`self.Warp2`) false)
  (bind _asmotion_controller_pawn (cast `/Game/VirtualRealityBP/Blueprints/MotionControllerPawn` (`GameplayStatics.GetPlayerPawn` 0)))
  (`self.K2_AddActorWorldOffset` _asmotion_controller_pawn (0.0 0.0 8000.0) false true)
  (`self.SetActorHiddenInGame` (`self.BP_stanza`) true)
  (`KismetSystemLibrary.Delay` 2.0)
  (`self.SetActorHiddenInGame` (`self.Landscape`) false)
  (`KismetSystemLibrary.Delay` 2.5)
  (bind _asmotion_controller_pawn_2 (cast `/Game/VirtualRealityBP/Blueprints/MotionControllerPawn` (`GameplayStatics.GetPlayerPawn` 0)))
  (`self.K2_AddActorWorldOffset` _asmotion_controller_pawn_2 (0.0 0.0 -8000.0) false true)
  ;[1 1 1] Respawn Drappo
  (`/Game/ABP/Drappo/BP_Drappo.Respawn` (`self.bp_drappo`))
  (`self.SetActorHiddenInGame` (`self.Warp1`) true)
  (`self.SetActorHiddenInGame` (`self.Warp2`) true))

(fn `UserConstructionScript`)