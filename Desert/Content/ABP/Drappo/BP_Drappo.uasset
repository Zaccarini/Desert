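; BP_Drappo is a drape actor that can be picked up by attaching to a component, then dropped to trigger a tent animation sequence.
; Drop detaches it and starts a fast looping timer that nudges it toward TargetDubai.
; After delays it hides, reveals and runs the TendaAnimata actors, then calls BPStart.SpawnInEnd and stops the timer.
; Separate events hide the animated tent and respawn the drape at TargetDrappo.
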(event `/Game/VirtualRealityBP/Blueprints/PickupActorInterface.Pickup`
  (params (AttachTo :type "SceneComponent Object Reference") (`Oculus Hand` :type "OculusHandComponent Object Reference"))
  (`self.K2_AttachToComponent` self AttachTo "None" "KeepWorld" "KeepWorld" "KeepRelative" true))

(event `/Game/VirtualRealityBP/Blueprints/PickupActorInterface.Drop`
  (`self.K2_DetachFromActor` "KeepWorld" "KeepWorld")
  (`KismetSystemLibrary.Delay` 0.2)
  (bind _returnvalue (`KismetSystemLibrary.K2_SetTimerDelegate` (delegate `MovingToDubai`) 0.005 true))
  (set `self.TimerToDubai` _returnvalue)
  (`KismetSystemLibrary.Delay` 2.0)
  (`KismetSystemLibrary.Delay` 1.0)
  (`self.SetActorHiddenInGame` true)
  (for _array_element (`self.TendaAnimata`)
    (set `GeometryCacheComponent.bRunning` true _array_element)
    (`SceneComponent.SetHiddenInGame` _array_element false false))
  ;[1 1 1] Delay Animazione Tenda
  (`KismetSystemLibrary.Delay` 7.0)
  (`/Game/ABP/StartButton/BP_Start.SpawnInEnd` (`self.BP_Start`))
  (`KismetSystemLibrary.K2_ClearAndInvalidateTimerHandle` (`self.TimerToDubai`)))

(event `MovingToDubai`
  (bind _returnvalue (`self.K2_GetActorLocation`))
  (`self.K2_SetActorLocation` (+ (`KismetMathLibrary.GetForwardVector` (`KismetMathLibrary.FindLookAtRotation` _returnvalue (`self.K2_GetActorLocation` (`self.TargetDubai`)))) _returnvalue)))

(event `TendaAnimataHide`
  (for _array_element (`self.TendaAnimata`)
    (set `GeometryCacheComponent.bRunning` false _array_element)
    (`SceneComponent.SetHiddenInGame` _array_element true false)))

(event `Respawn`
  (`self.K2_SetActorLocation` (`self.K2_GetActorLocation` (`self.TargetDrappo`)))
  (`self.SetActorHiddenInGame` false))

(fn `UserConstructionScript`)