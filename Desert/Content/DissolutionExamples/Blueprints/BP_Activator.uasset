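; BP_Activator is an overlap trigger that tells a list of target actors to play an appearance or dissolve effect.
; Entering the sphere changes the decal color, hides the text label and messages each target in turn, optionally staggered by Duration through a manually advanced loop.
; Leaving restores the visuals, breaks the loop and sends every target a deactivate message.
; The construction script sets the label from the Appearance flag.
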(event `self.ReceiveBeginPlay`
  (bind _returnvalue (`KismetMaterialLibrary.CreateDynamicMaterialInstance` "/Game/DissolutionExamples/Materials/MI_ActivatorDecalMaterial_Inst.MI_ActivatorDecalMaterial_Inst"))
  (bind _output_get (set `self.DecalMaterial` _returnvalue))
  (`DecalComponent.SetDecalMaterial` (`self.Decal`) _output_get))

(event `self.Sphere.OnComponentBeginOverlap`
  (params (OverlappedComponent :type "PrimitiveComponent Object Reference") (OtherActor :type "Actor Object Reference") (OtherComp :type "PrimitiveComponent Object Reference") (OtherBodyIndex :type Integer) (bFromSweep :type Boolean) (SweepResult :type "HitResult Structure (by ref)"))
  (`self.Activate` (`self.Appearance`)))

(event `self.Sphere.OnComponentEndOverlap`
  (params (OverlappedComponent :type "PrimitiveComponent Object Reference") (OtherActor :type "Actor Object Reference") (OtherComp :type "PrimitiveComponent Object Reference") (OtherBodyIndex :type Integer))
  (`self.Deactivate`))

(event `self.Activate`
  (params (Appearance :type Boolean))
  (bind _duration (`self.Duration`))
  (`MaterialInstanceDynamic.SetVectorParameterValue` (`self.DecalMaterial`) "Color" (struct :`A` 1.0))
  (`SceneComponent.SetVisibility` (`self.TextRender`) false false)
  (bind _arrayelement (`/Game/DissolutionExamples/Blueprints/MacroLibrary/BP_LoopMacroLibrary.OpenForeachLoopWithBreak` (`self.TargetActors`) :!via `Exec` :!label _label)
    (:`LoopBody`
      (`|ExecutionSequence`
        (:`then_0`
          (`/Engine/EditorBlueprintResources/StandardMacros.IsValid` _arrayelement
            (:`Is Valid`
              (message `/Game/DissolutionExamples/Blueprints/Interface/BP_ActivationInterface.Activate` _arrayelement Appearance))))
        (:`then_1`
          (if (> _duration 0.0)
            (`KismetSystemLibrary.RetriggerableDelay` _duration)
            (goto _label)
            (else
              (goto _label))))))))

(event `self.Deactivate`
  (`MaterialInstanceDynamic.SetVectorParameterValue` (`self.DecalMaterial`) "Color" (struct :`R` 1.0 :`A` 1.0))
  (`SceneComponent.SetVisibility` (`self.TextRender`) true false)
  (`|ExecutionSequence`
    (:`then_0`
      (goto _label :!via `Break`))
    (:`then_1`
      (for _array_element (`self.TargetActors`)
        (`/Engine/EditorBlueprintResources/StandardMacros.IsValid` _array_element
          (:`Is Valid`
            (message `/Game/DissolutionExamples/Blueprints/Interface/BP_ActivationInterface.Deactivate` _array_element)))))))

(fn `UserConstructionScript`
  (`TextRenderComponent.K2_SetText` (`self.TextRender`) (`KismetTextLibrary.Conv_StringToText` (select `bool` (`self.Appearance`) :`false` "Activate Dissolve" :`true` "Activate Appearance"))))