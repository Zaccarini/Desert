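; Dissolver child Blueprint that spawns Niagara dissolve effects for an actor's static and skeletal meshes, including those on attached actors.
; Its Dissolve override gathers the mesh components, then creates one auto-destroying Niagara component per mesh from the supplied system.
; Each effect receives the mesh, its slot 0 material, the dissolver's location as center and a lifetime.
; It returns the spawned components; activation and deactivation defer to the parent.
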(event `/Game/DissolutionExamples/Blueprints/Interface/BP_ActivationInterface.Activate`
  (params (Appearance :type Boolean))
  (`parent.Activate` Appearance))

(event `/Game/DissolutionExamples/Blueprints/Interface/BP_ActivationInterface.Deactivate`
  (`parent.Deactivate`))

(fn `Dissolve`
  (params (Actor :type "Actor Object Reference") (InAsset :type "NiagaraSystem Object Reference"))
  (returns (NiagaraComponents :type "Array of NiagaraComponent Object Reference"))
  (locals (LocalNiagaraComponents :type "Array of NiagaraComponent Object Reference") (LocalComponents :type "Array of PrimitiveComponent Object Reference"))
  (bind _actor (`local.Actor`))
  (bind _localcomponents (`local.LocalComponents`))
  (bind _actor_2 (`local.Actor`))
  (bind _returnvalue (`self.K2_GetComponentsByClass` _actor_2 "/Script/Engine.SkeletalMeshComponent"))
  (bind _returnvalue_2 (`self.K2_GetComponentsByClass` _actor "/Script/Engine.StaticMeshComponent"))
  (`/Engine/EditorBlueprintResources/StandardMacros.IsValid` Actor
    (:`Is Valid`
      (`/Engine/EditorBlueprintResources/StandardMacros.IsValid` InAsset
        (:`Is Valid`
          (`|ExecutionSequence`
            (:`then_0`
              (`|ExecutionSequence`
                (:`then_0`
                  (if (> (`KismetArrayLibrary.Array_Length` _returnvalue_2) 0)
                    (`KismetArrayLibrary.Array_Append` _localcomponents _returnvalue_2)))
                (:`then_1`
                  (for _array_element (`self.GetAttachedActors` _actor true)
                    (bind _returnvalue_3 (`self.K2_GetComponentsByClass` _array_element "/Script/Engine.StaticMeshComponent"))
                    (if (> (`KismetArrayLibrary.Array_Length` _returnvalue_3) 0)
                      (`KismetArrayLibrary.Array_Append` (`local.LocalComponents`) _returnvalue_3))))))
            (:`then_1`
              (`|ExecutionSequence`
                (:`then_0`
                  (if (> (`KismetArrayLibrary.Array_Length` _returnvalue) 0)
                    (`KismetArrayLibrary.Array_Append` _localcomponents _returnvalue)))
                (:`then_1`
                  (for _array_element_2 (`self.GetAttachedActors` _actor_2 true)
                    (bind _returnvalue_4 (`self.K2_GetComponentsByClass` _array_element_2 "/Script/Engine.SkeletalMeshComponent"))
                    (if (> (`KismetArrayLibrary.Array_Length` _returnvalue_4) 0)
                      (`KismetArrayLibrary.Array_Append` (`local.LocalComponents`) _returnvalue_4))))))
            (:`then_2`
              (for _array_element_3 (`local.LocalComponents`)
                (`|ExecutionSequence`
                  (:`then_0`
                    (bind _returnvalue_5 (`AddComponent|NODE_AddNiagaraComponent-0` :`bManualAttachment` true :`RelativeTransform` (`KismetMathLibrary.Conv_VectorToTransform` (`self.K2_GetActorLocation` (`local.Actor`)))))
                    (`KismetArrayLibrary.Array_Add` (`local.LocalNiagaraComponents`) _returnvalue_5)
                    (`NiagaraComponent.SetAsset` _returnvalue_5 (`local.InAsset`))
                    (`NiagaraComponent.SetVariableMaterial` _returnvalue_5 "Material" (`PrimitiveComponent.GetMaterial` _array_element_3 0))
                    (`NiagaraComponent.SetVariableVec3` _returnvalue_5 "Center" (`self.K2_GetActorLocation`))
                    (`NiagaraComponent.SetNiagaraVariableFloat` _returnvalue_5 "Lifetime" (`self.Lifetime`))
                    (`NiagaraComponent.SetAutoDestroy` _returnvalue_5 true))
                  (:`then_1`
                    (bind _asstatic_mesh_component (cast `StaticMeshComponent` _array_element_3))
                    (`NiagaraFunctionLibrary.OverrideSystemUserVariableStaticMeshComponent` _returnvalue_5 "StaticMesh" _asstatic_mesh_component))
                  (:`then_2`
                    (bind _asskeletal_mesh_component (cast `SkeletalMeshComponent` _array_element_3))
                    (`NiagaraFunctionLibrary.OverrideSystemUserVariableSkeletalMeshComponent` _returnvalue_5 "SkeletalMesh" _asskeletal_mesh_component))
                  (:`then_3`
                    (`ActorComponent.Activate` _returnvalue_5 true)))))
            (:`then_4`
              (return (`local.LocalNiagaraComponents`)))))
        (:`Is Not Valid`
          (return (`local.LocalNiagaraComponents`)))))
    (:`Is Not Valid`
      (return (`local.LocalNiagaraComponents`)))))

(fn `UserConstructionScript`
  (`parent.UserConstructionScript`))